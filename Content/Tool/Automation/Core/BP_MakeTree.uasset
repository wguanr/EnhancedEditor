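; Spline placement tool that lines a path with trees or road lamps as instances of a chosen mesh.
; The construction script fills a Hierarchical Instanced Static Mesh at intervals of the mesh's X bounds plus extra spacing.
; Road lamp mode aims each instance at the next point.
; Tree mode uses the sine of the index for deterministic variation in yaw and height.
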(fn `Get Location at Index`
  (params (A :type Integer))
  (returns (ReturnValue :type "Vector Structure"))
  (return (`SplineComponent.GetLocationAtDistanceAlongSpline` (`self.Spline`) (* A (`self.setDistance`)) "Local")))

(fn `set Distance and Unit`
  (params (Unit :type "StaticMesh Object Reference") (Space :type "Float (double-precision)"))
  (returns (Index :type Boolean) (distance :type "Float (double-precision)"))
  (bind (_min _max) (break `Box` (`StaticMesh.GetBoundingBox` Unit)))
  (bind _returnvalue (`StaticMeshComponent.SetStaticMesh` (`self.HierarchicalInstancedStaticMesh`) Unit))
  (return _returnvalue (+ (.x (- _max _min)) Space)))

(fn `UserConstructionScript`
  (locals (count :type Integer :default 0))
  (bind _distance (`self.Distance`))
  (bind _unit (`self.Unit`))
  (bind (_x _y _z) (`KismetMathLibrary.BreakVector3f` (`self.Scale`)))
  (if (`self.change to RoadLamp?`)
    (bind (_index _distance_2) (`self.set Distance and Unit` _unit _distance))
    (bind _output_get (set `self.setDistance` _distance_2))
    (for _index_2 (range (+ (`KismetMathLibrary.FFloor` (/ (`SplineComponent.GetSplineLength` (`self.Spline`)) _output_get)) 1))
      (bind _returnvalue (`self.Get Location at Index` _index_2))
      (`InstancedStaticMeshComponent.AddInstance` (`self.HierarchicalInstancedStaticMesh`) (`KismetMathLibrary.MakeTransform` _returnvalue (`KismetMathLibrary.MakeRotFromX` (- (`self.Get Location at Index` (+ _index_2 1)) _returnvalue)) (`self.Scale`)) false))
    (else
      (bind (_index_3 _distance_3) (`self.set Distance and Unit` _unit _distance))
      (bind _output_get_2 (set `self.setDistance` _distance_3))
      (for _index_4 (range (+ (`KismetMathLibrary.FFloor` (/ (`SplineComponent.GetSplineLength` (`self.Spline`)) _output_get_2)) 1))
        (bind _returnvalue_2 (`KismetMathLibrary.Sin` (`KismetMathLibrary.Conv_IntToDouble` _index_4)))
        (`InstancedStaticMeshComponent.AddInstance` (`self.HierarchicalInstancedStaticMesh`) (`KismetMathLibrary.MakeTransform` (`self.Get Location at Index` _index_4) (`KismetMathLibrary.MakeRotator` 0.0 0.0 (* 120 _returnvalue_2)) (`KismetMathLibrary.MakeVector` _x _y (`KismetMathLibrary.MapRangeClamped` _returnvalue_2 0.0 1.0 (* _z 0.9) _z))) false)))))